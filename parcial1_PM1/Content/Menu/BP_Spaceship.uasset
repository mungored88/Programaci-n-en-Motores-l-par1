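; BP_Spaceship is a spaceship actor in the Menu folder that drifts slowly forward along its own facing.
; Each Tick it lerps from its location toward a point just ahead, giving a small fixed step per frame that is not scaled by delta time and does not sweep for collision.
; A forward visibility line trace with debug drawing is present but disconnected, so it never runs.
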(event `self.ReceiveTick`
  (params (DeltaSeconds :type "Float (single-precision)"))
  (bind _returnvalue (`self.K2_GetActorLocation`))
  (`self.K2_SetActorLocation` (`KismetMathLibrary.VLerp` _returnvalue (+ _returnvalue (* (`KismetMathLibrary.GetForwardVector` (`self.K2_GetActorRotation`)) 0.3)) 0.1)))

(event `self.ReceiveBeginPlay`)

(fn `UserConstructionScript`)