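; BP_AlienShoot is a shooting alien enemy that pursues the FirstPersonCharacter and fires at it while its health remains.
; Tick calls WidgetLookCam and reissues AIMoveTo toward the player, stopping movement once health runs out.
; A three-second Delay, reached from Tick and move success, paces a forward line trace with laser sound and muzzle effect.
; A hit on the player applies damage and spawns blood at the impact point.
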(event `self.ReceiveBeginPlay`
  (`parent.ReceiveBeginPlay`))

(event `self.ReceiveTick`
  (params (DeltaSeconds :type "Float (single-precision)"))
  (bind _linetracestart (`self.LineTraceStart`))
  (bind _returnvalue (`SceneComponent.K2_GetComponentLocation` (`self.LineTraceStart`)))
  (bind _returnvalue_2 (`SceneComponent.K2_GetComponentLocation` _linetracestart))
  (`self.WidgetLookCam` false)
  (if (> (`self.Health`) 0.1)
    (bind _returnvalue_3 (`GameplayStatics.GetActorOfClass` "/Game/FirstPersonBP/Blueprints/FirstPersonCharacter.FirstPersonCharacter_C"))
    (`|AIMoveTo` self (`self.K2_GetActorLocation` _returnvalue_3) null
      (:`then`
        _)
      (:`OnSuccess`
        _))
    (`KismetSystemLibrary.Delay` 3.0)
    (bind _outhit (`KismetSystemLibrary.LineTraceSingle` _returnvalue_2 (+ _returnvalue_2 (* (`SceneComponent.GetForwardVector` _linetracestart) 5000.0)) "TraceTypeQuery1"))
    (`GameplayStatics.SpawnSoundAtLocation` "/Game/Sounds/376694__daleonfire__laserShot.376694__daleonfire__laserShot" _returnvalue (struct) 0.1 1.0 0.0 "/Game/Sounds/EnemyAttenuation.EnemyAttenuation" null)
    (`GameplayStatics.SpawnEmitterAtLocation` "/Game/StarterContent/Particles/P_Explosion.P_Explosion" _returnvalue (struct) (0.1 0.1 0.1))
    (bind (_bblockinghit _binitialoverlap _time _distance _location _impactpoint _normal _impactnormal _physmat _hitactor) (`GameplayStatics.BreakHitResult` _outhit))
    (bind _asfirst_person_character (cast `/Game/FirstPersonBP/Blueprints/FirstPersonCharacter` _hitactor))
    (`/Game/FirstPersonBP/Blueprints/FirstPersonCharacter.Damage` _asfirst_person_character (`self.DamageAplicateInPlayer`))
    (`GameplayStatics.SpawnEmitterAtLocation` "/Game/Otros/FXVillesBloodVFXPack/Particles/PS_Blood_Slice.PS_Blood_Slice" _location)
    (else
      (`MovementComponent.StopMovementImmediately` (`self.CharacterMovement`)))))

(fn `UserConstructionScript`
  (`parent.UserConstructionScript`))