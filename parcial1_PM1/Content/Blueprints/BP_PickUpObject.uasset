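; BP_PickUpObject is a collectible that spins in place and awards a point when the first-person character touches it.
; Tick adds a fixed local rotation each frame, not scaled by delta time.
; Sphere overlap increments the character's Points, prints the total, spawns an explosion particle and a collect sound, updates the score on the player's UI, then destroys the pickup.
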(event `self.ReceiveTick`
  (params (DeltaSeconds :type "Float (single-precision)"))
  ;[1 0.6367 0.5667] -Object Rotation
  (`self.K2_AddActorLocalRotation` (struct :`Yaw` 4.0)))

(event `self.Sphere.OnComponentBeginOverlap`
  (params (OverlappedComponent :type "PrimitiveComponent Object Reference") (OtherActor :type "Actor Object Reference") (OtherComp :type "PrimitiveComponent Object Reference") (OtherBodyIndex :type Integer) (bFromSweep :type Boolean) (SweepResult :type "HitResult Structure (by ref)"))
  ;[0.8366 0.4797 1] -Pick up Events
  (bind _asfirst_person_character (cast `/Game/FirstPersonBP/Blueprints/FirstPersonCharacter` OtherActor))
  ;;[1 1 1] Set Points and Display it
  (bind _output_get (set `/Game/FirstPersonBP/Blueprints/FirstPersonCharacter.Points` (+ (`/Game/FirstPersonBP/Blueprints/FirstPersonCharacter.Points` _asfirst_person_character) 1) _asfirst_person_character))
  (`KismetSystemLibrary.PrintString` (`KismetStringLibrary.Conv_IntToString` _output_get))
  ;;[1 1 1] Particle
  (`GameplayStatics.SpawnEmitterAtLocation` "/Game/StarterContent/Particles/P_Explosion.P_Explosion" (`self.K2_GetActorLocation`))
  ;;[1 1 1] Sound
  (`GameplayStatics.SpawnSoundAtLocation` "/Game/Sounds/499790__robinhood76__08470-music-box-collect-ding.499790__robinhood76__08470-music-box-collect-ding" (`self.K2_GetActorLocation`) (struct) 1.0 1.0 0.0 null null)
  (`/Game/UI/UI_Score.Update_Score` (`/Game/FirstPersonBP/Blueprints/FirstPersonCharacter.UIPlayer` _asfirst_person_character) _output_get)
  (`self.K2_DestroyActor`))

(fn `UserConstructionScript`)