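; Enemy spawner actor that repeatedly spawns an Enemies actor at one of three points marked by its Arrow components.
; BeginPlay caches the arrows' world locations in a Position array.
; Tick feeds a random 10 to 40 second Delay, which ignores re-triggers while pending and so acts as a repeating timer.
; Each time it completes, a spawn happens at a randomly chosen cached location.
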(event `self.ReceiveBeginPlay`
  (bind _position (`self.Position`))
  (`KismetArrayLibrary.Array_Add` _position (`SceneComponent.K2_GetComponentLocation` (`self.Arrow`)))
  (`KismetArrayLibrary.Array_Add` _position (`SceneComponent.K2_GetComponentLocation` (`self.Arrow1`)))
  (`KismetArrayLibrary.Array_Add` _position (`SceneComponent.K2_GetComponentLocation` (`self.Arrow2`))))

(event `self.ReceiveTick`
  (params (DeltaSeconds :type "Float (single-precision)"))
  (`KismetSystemLibrary.Delay` (`KismetMathLibrary.RandomFloatInRange` 10.0 40.0))
  (`|SpawnActorFromClass` (`self.Enemies`) (`KismetMathLibrary.MakeTransform` (`|GetArrayItem` (`self.Position`) (`KismetMathLibrary.RandomIntegerInRange` 0 2))) "Undefined" "OverrideRootScale" null null))

(fn `UserConstructionScript`)