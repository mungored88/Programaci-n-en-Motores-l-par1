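; BP_AlienRock is a rock-disguised alien enemy that pursues the FirstPersonCharacter while Health remains, and stops moving otherwise.
; Tick resets it to invulnerable with rock materials, then issues AI moves to the player.
; Reaching the Distance radius sets IsVulnerable and swaps in alien body materials.
; Reaching the closer radius plays an attenuated monster sound and pauses the walk animation briefly through its AnimInstance.
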(event `self.ReceiveTick`
  (params (DeltaSeconds :type "Float (single-precision)"))
  (bind _mesh (`self.Mesh`))
  (bind _mesh_2 (`self.Mesh`))
  (set `self.IsVulnerable` false)
  (`PrimitiveComponent.SetMaterial` _mesh 0 "/Game/StarterContent/Props/Materials/M_Rock.M_Rock")
  (`PrimitiveComponent.SetMaterial` _mesh 1 "/Game/StarterContent/Props/Materials/M_Rock.M_Rock")
  (`self.WidgetLookCam` false)
  (if (> (`self.Health`) 0.0)
    (bind _returnvalue (`GameplayStatics.GetActorOfClass` "/Game/FirstPersonBP/Blueprints/FirstPersonCharacter.FirstPersonCharacter_C"))
    (bind _returnvalue_2 (`self.K2_GetActorLocation` _returnvalue))
    (`|AIMoveTo` self _returnvalue_2 null (`self.Distance`)
      (:`then`
        _)
      (:`OnSuccess`
        (set `self.IsVulnerable` true)
        (`PrimitiveComponent.SetMaterial` _mesh_2 0 "/Game/Models/Materials/AlienTeleporter2_body.AlienTeleporter2_body")
        (`PrimitiveComponent.SetMaterial` _mesh_2 1 "/Game/Models/Materials/AlienTeleporter_body.AlienTeleporter_body")))
    (`|AIMoveTo` self _returnvalue_2 null 100.0
      (:`OnSuccess`
        (`GameplayStatics.SpawnSoundAtLocation` "/Game/Sounds/monster.monster" (`SceneComponent.K2_GetComponentLocation` (`self.Mesh`)) (struct) 0.15 1.0 0.0 "/Game/Sounds/EnemyAttenuation.EnemyAttenuation" null)
        (bind _asbp_animation_alien_rock (cast `/Game/Models/BluePrint_enemies/BP_Animation_AlienRock` (`SkeletalMeshComponent.GetAnimInstance` (`self.Mesh`))))
        (set `/Game/Models/BluePrint_enemies/BP_Animation_AlienRock.ParamWalk` false _asbp_animation_alien_rock)
        (`KismetSystemLibrary.Delay` 1.0)
        (set `/Game/Models/BluePrint_enemies/BP_Animation_AlienRock.ParamWalk` true _asbp_animation_alien_rock)))
    (else
      (`MovementComponent.StopMovementImmediately` (`self.CharacterMovement`)))))

(fn `UserConstructionScript`
  (`parent.UserConstructionScript`))