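; BP_AlienExperiment is an enemy character that chases the player while its health is above zero.
; Each Tick it updates WidgetLookCam and issues AIMoveTo toward the FirstPersonCharacter's location, stopping movement once health runs out.
; On arrival it jumps and clears the anim blueprint's ParamWalkE flag for a short delay.
; The Asd function spawns a BP_Hit_Damage actor at the Hit component, passing it the player damage value.
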(event `self.ReceiveTick`
  (params (DeltaSeconds :type "Float (single-precision)"))
  (`self.WidgetLookCam` false)
  (if (> (`self.Health`) 0.0)
    (bind _returnvalue (`GameplayStatics.GetActorOfClass` "/Game/FirstPersonBP/Blueprints/FirstPersonCharacter.FirstPersonCharacter_C"))
    (`|AIMoveTo` self (`self.K2_GetActorLocation` _returnvalue) null (`self.Distance`)
      (:`OnSuccess`
        (bind _asbp_animation_alien_experiment (cast `/Game/Models/BluePrint_enemies/BP_Animation_AlienExperiment` (`SkeletalMeshComponent.GetAnimInstance` (`self.Mesh`))))
        (set `/Game/Models/BluePrint_enemies/BP_Animation_AlienExperiment.ParamWalkE` false _asbp_animation_alien_experiment)
        (`self.Jump`)
        (`KismetSystemLibrary.Delay` 2.0)
        (set `/Game/Models/BluePrint_enemies/BP_Animation_AlienExperiment.ParamWalkE` true _asbp_animation_alien_experiment)))
    (else
      (`MovementComponent.StopMovementImmediately` (`self.CharacterMovement`)))))

(fn `asd`
  (bind _hit (`self.Hit`))
  (bind _returnvalue (`|SpawnActorFromClass` "/Game/Models/BluePrint_enemies/BP_Hit_Damage.BP_Hit_Damage_C" (`KismetMathLibrary.MakeTransform` (`SceneComponent.K2_GetComponentLocation` _hit) (`SceneComponent.K2_GetComponentRotation` _hit)) "Undefined" "OverrideRootScale" null null))
  (set `/Game/Models/BluePrint_enemies/BP_Hit_Damage.Damages` (`self.DamageAplicateInPlayer`) _returnvalue))

(fn `UserConstructionScript`
  (`parent.UserConstructionScript`))