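; BP_Alien is an enemy character that chases the player's FirstPersonCharacter.
; Each Tick it issues an AI move, and on arrival plays a monster sound and briefly clears the animation Blueprint's walk flag.
; Damage updates a camera-facing health widget; at zero health the mesh ragdolls, then the actor is destroyed after a delay.
; GenerationHit, not called within this Blueprint, spawns a damage actor carrying the player-damage value.
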(event `self.ReceiveBeginPlay`
  (set `CharacterMovementComponent.MaxWalkSpeed` (`self.MaxSpeed`) (`self.CharacterMovement`)))

(event `self.ReceiveTick`
  (params (DeltaSeconds :type "Float (single-precision)"))
  (`self.WidgetLookCam` false)
  (if (> (`self.Health`) 0.1)
    (bind _returnvalue (`GameplayStatics.GetActorOfClass` "/Game/FirstPersonBP/Blueprints/FirstPersonCharacter.FirstPersonCharacter_C"))
    (`|AIMoveTo` self (`self.K2_GetActorLocation` _returnvalue) null (`self.Distance`)
      (:`OnSuccess`
        (`GameplayStatics.SpawnSoundAtLocation` "/Game/Sounds/monster.monster" (`SceneComponent.K2_GetComponentLocation` (`self.Mesh`)) (struct) 1.0 1.0 0.0 null null)
        (bind _asbp_animation_alien (cast `/Game/Models/BluePrint_enemies/BP_Animation_Alien` (`SkeletalMeshComponent.GetAnimInstance` (`self.Mesh`))))
        (set `/Game/Models/BluePrint_enemies/BP_Animation_Alien.ParamWalk` false _asbp_animation_alien)
        (`KismetSystemLibrary.Delay` 0.2)
        (set `/Game/Models/BluePrint_enemies/BP_Animation_Alien.ParamWalk` true _asbp_animation_alien)))
    (else
      (`MovementComponent.StopMovementImmediately` (`self.CharacterMovement`)))))

(event `Damage`
  (params (DamageAmount :type "Float (double-precision)"))
  (bind _output_get (set `self.Health` (`KismetMathLibrary.FClamp` (- (`self.Health`) DamageAmount) 0.0 100.0)))
  (bind _asui_life_enemy (cast `/Game/UI/UI_Life_Enemy` (`WidgetComponent.GetWidget` (`self.Widget_Life_Enemy`))))
  (`/Game/UI/UI_Life_Enemy.UpdateLife` _asui_life_enemy (`self.Health`) 100.0)
  (if (== _output_get 0.0)
    (`SkeletalMeshComponent.SetAllBodiesSimulatePhysics` (`self.Mesh`) true)
    (`PrimitiveComponent.SetCollisionEnabled` (`self.CapsuleComponent`) "NoCollision")
    (`PrimitiveComponent.SetCollisionEnabled` (`self.Mesh`) "QueryAndPhysics")
    (`KismetSystemLibrary.Delay` 7.0)
    (`self.K2_DestroyActor`)))

(fn `GenerationHit`
  (bind _hit (`self.Hit`))
  (bind _returnvalue (`|SpawnActorFromClass` "/Game/Models/BluePrint_enemies/BP_Hit_Damage.BP_Hit_Damage_C" (`KismetMathLibrary.MakeTransform` (`SceneComponent.K2_GetComponentLocation` _hit) (`SceneComponent.K2_GetComponentRotation` _hit)) "Undefined" "OverrideRootScale" null null))
  (set `/Game/Models/BluePrint_enemies/BP_Hit_Damage.Damages` (`self.DamageAplicateInPlayer`) _returnvalue))

(fn `UserConstructionScript`)

(fn `WidgetLookCam`
  (params (NewParam :type Boolean))
  (`SceneComponent.K2_SetWorldRotation` (`self.Widget_Life_Enemy`) (`KismetMathLibrary.MakeRotator` 0.0 0.0 (.yaw (`KismetMathLibrary.FindLookAtRotation` (`SceneComponent.K2_GetComponentLocation` (`self.Widget_Life_Enemy`)) (`PlayerCameraManager.GetCameraLocation` (`GameplayStatics.GetPlayerCameraManager` 0))))) false false))