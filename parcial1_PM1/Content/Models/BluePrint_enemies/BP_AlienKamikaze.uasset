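; BP_AlienKamikaze is a suicide enemy that chases the first-person character and explodes on reaching it.
; While Health remains, every Tick re-issues AI MoveTo toward the player's location, with a delayed monster sound on the side.
; A successful move spawns an explosion, damages the player and destroys the alien shortly after.
; Tick also calls WidgetLookCam, and halts movement once Health runs out.
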(event `self.ReceiveTick`
  (params (DeltaSeconds :type "Float (single-precision)"))
  (`self.WidgetLookCam` false)
  (if (> (`self.Health`) 0.1)
    (bind _returnvalue (`GameplayStatics.GetActorOfClass` "/Game/FirstPersonBP/Blueprints/FirstPersonCharacter.FirstPersonCharacter_C"))
    (`|AIMoveTo` self (`self.K2_GetActorLocation` _returnvalue) null (`self.Distance`)
      (:`then`
        (`KismetSystemLibrary.Delay` 10.0)
        (`GameplayStatics.SpawnSoundAtLocation` "/Game/Sounds/monster.monster" (`SceneComponent.K2_GetComponentLocation` (`self.Mesh`)) (struct) 0.15 1.0 0.0 "/Game/Sounds/EnemyAttenuation.EnemyAttenuation" null))
      (:`OnSuccess`
        (`GameplayStatics.SpawnEmitterAtLocation` "/Game/StarterContent/Particles/P_Explosion.P_Explosion" (`SceneComponent.K2_GetComponentLocation` (`self.Mesh`)) (struct) (5.0 5.0 5.0))
        (bind _asfirst_person_character (cast `/Game/FirstPersonBP/Blueprints/FirstPersonCharacter` _returnvalue))
        (`/Game/FirstPersonBP/Blueprints/FirstPersonCharacter.Damage` _asfirst_person_character (`self.DamageAplicateInPlayer`))
        (`KismetSystemLibrary.Delay` 0.5)
        (`self.K2_DestroyActor`)))
    (else
      (`MovementComponent.StopMovementImmediately` (`self.CharacterMovement`)))))

(fn `UserConstructionScript`
  (`parent.UserConstructionScript`))